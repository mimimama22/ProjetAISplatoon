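; Base AI controller for BP_AIBase pawns in a two-team game, choosing a gun or brush behavior tree by whether the pawn has a pistol.
; On possess it writes the opposing team's spawn base to the blackboard.
; AI perception stores sensed enemies as blackboard objects and sets a bool, apparently for fleeing ("Fuyer"), when exactly one enemy is in an update.
; The spline lookup logic is unconnected.
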(event OnPerceptionUpdated(AIPerception)
  (params (UpdatedActors :type Array%20of%20Actor%20Object%20References))
  (Utilities|Array|Clear (Variables|Default|GetArrayEnemyDetected))
  (Variables|Default|SetArray%20Index 0)
  (for _array_element UpdatedActors
    (bind _asbp_aibase (Utilities|Casting|CastToBP_AIBase _array_element))
    (if (!= (Variables|/Game/GameCore/Blueprint/AI/BP_AIBase.BP_AIBase_C|GetIsTeamRed _asbp_aibase) (Variables|/Game/GameCore/Blueprint/AI/BP_AIBase.BP_AIBase_C|GetIsTeamRed (Variables|Default|GetAs%20BP%20AIBase)))
      (Math|Integer|IncrementInt (Variables|Default|GetArray%20Index)
        (:%20%20
          (Utilities|Array|Add (Variables|Default|GetArrayEnemyDetected) _asbp_aibase)))))
  (if (== (Variables|Default|GetArray%20Index) 1)
    (Development|PrintString "Fuyer" true true "(R=0.000000,G=0.000000,B=0.000000,A=1.000000)")
    (AI|Components|Blackboard|SetValueasBool (Variables|Default|GetBlackboard) (Variables|Default|GetKey%20Name_1) true)
    (else
      (AI|Components|Blackboard|SetValueasBool (Variables|Default|GetBlackboard) (Variables|Default|GetKey%20Name_1) false))))

(event OnTargetPerceptionUpdated(AIPerception)
  (params (Actor :type Actor%20Object%20Reference) (Stimulus :type AI%20Stimulus%20Structure))
  (bind _asbp_aibase (Utilities|Casting|CastToBP_AIBase Actor))
  (if (!= (Variables|/Game/GameCore/Blueprint/AI/BP_AIBase.BP_AIBase_C|GetIsTeamRed _asbp_aibase) (Variables|/Game/GameCore/Blueprint/AI/BP_AIBase.BP_AIBase_C|GetIsTeamRed (Variables|Default|GetAs%20BP%20AIBase)))
    (AI|Components|Blackboard|SetValueasObject (Variables|Default|GetBlackboard) (Variables|Default|GetKey%20Name) _asbp_aibase)))

(event EventBeginPlay)

(event EventPossess
  (params (PossessedPawn :type Pawn%20Object%20Reference))
  (bind _asbp_aibase (Utilities|Casting|CastToBP_AIBase PossessedPawn))
  (bind _output_get (Variables|Default|SetAs%20BP%20AIBase _asbp_aibase))
  (Variables|/Game/GameCore/Blueprint/AI/BP_AIBase.BP_AIBase_C|SetRef_AIC _output_get self)
  (if (Variables|/Game/GameCore/Blueprint/AI/BP_AIBase.BP_AIBase_C|GetHasPistol _output_get)
    (AI|RunBehaviorTree "/Game/GameCore/Blueprint/AI/BT_AIGun.BT_AIGun")
    (else
      (AI|RunBehaviorTree "/Game/GameCore/Blueprint/AI/BT_AIBrush.BT_AIBrush")))
  (bind _outactors (Actor|GetAllActorsOfClass "/Game/GameCore/Blueprint/Base/BP_SpawnBaseTeam.BP_SpawnBaseTeam_C"))
  (for _array_element _outactors
    (bind _as_bp_aibase (Variables|Default|GetAs%20BP%20AIBase)
      (:then
        (if (!= (Variables|/Game/GameCore/Blueprint/Base/BP_SpawnBaseTeam.BP_SpawnBaseTeam_C|GetIsTeamRed _array_element) (Variables|/Game/GameCore/Blueprint/AI/BP_AIBase.BP_AIBase_C|GetIsTeamRed _as_bp_aibase))
          (bind _output_get_2 (Variables|Default|SetEnemi%20Base _array_element))
          (AI|Components|Blackboard|SetValueasObject (Variables|Default|GetBlackboard) (Variables|Default|GetKey%20Name_0) _output_get_2)))
      (:else))))

(fn ConstructionScript)