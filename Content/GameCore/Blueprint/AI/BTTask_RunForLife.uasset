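; Behavior Tree task, named as a flee action, that applies movement input to an AI pawn relative to detected enemies.
; All logic runs on Receive Abort AI, averaging AIC_Base's detected-enemy locations and taking the look-at direction from there to the pawn.
; That direction is negated, so the single movement input points toward the enemies.
; It calls FinishExecute, failing if the controller cast fails, and prints debug text.
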(event EventReceiveAbortAI
  (params (OwnerController :type AI%20Controller%20Object%20Reference) (ControlledPawn :type Pawn%20Object%20Reference))
  (Development|PrintString "test")
  (bind _asaic_base (Utilities|Casting|CastToAIC_Base OwnerController)
    (:then
      (bind _returnvalue (Class|GameplayStatics|GetActorArrayAverageLocation (Variables|/Game/GameCore/Blueprint/AI/AIC_Base.AIC_Base_C|GetArrayEnemyDetected _asaic_base)))
      (Development|PrintText (Utilities|Text|FormatText "Actor : {A} 
Average : {B}" (Utilities|String|ToString(Vector) (Transformation|GetActorForwardVector ControlledPawn)) (Utilities|String|ToString(Vector) (Math|Vector|GetForwardVector (Math|Rotator|FindLookatRotation _returnvalue (Transformation|GetActorLocation ControlledPawn))))))
      (Pawn|Input|AddMovementInput ControlledPawn (* (Math|Vector|GetForwardVector (Math|Rotator|FindLookatRotation _returnvalue (Transformation|GetActorLocation ControlledPawn))) -1.0) 1.0 false)
      (AI|BehaviorTree|FinishExecute true))
    (:CastFailed
      (Development|PrintString "failled")
      (AI|BehaviorTree|FinishExecute false))))