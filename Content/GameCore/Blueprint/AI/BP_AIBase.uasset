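; Base AI character for a two-team paint shooter, with team materials, splat color materials, brush painting and an ammo counter.
; BeginPlay applies team visuals, builds both teams' dynamic splat materials and starts a looping timer.
; RespawnSystem, guarded by a DoOnce, leaves a paint decal, parks the AI off-map, clears blackboard values and starts a cooldown timer that lengthens each death.
; Respawn restores walking, moves it above its base and resets the guard.
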(event Custom|InitColorPainting
  (params (Team :type Boolean))
  (bind _returnvalue (Rendering|Material|CreateDynamicMaterialInstance "/Game/Market/GunSplatoon/MI_ShootSplat.MI_ShootSplat" "None" "None" :!class /Script/Engine.KismetMaterialLibrary))
  (bind _output_get (Variables|Default|SetPainting _returnvalue))
  (Rendering|Material|SetVectorParameterValue _output_get "color" (select Team "(R=1.000000,G=0.000000,B=0.012401,A=1.000000)" "(R=0.000000,G=0.024492,B=1.000000,A=1.000000)") :!class /Script/Engine.MaterialInstanceDynamic)
  (bind _returnvalue_2 (Rendering|Material|CreateDynamicMaterialInstance "/Game/Market/GunSplatoon/MI_ShootSplat.MI_ShootSplat" "None" "None" :!class /Script/Engine.KismetMaterialLibrary))
  (bind _output_get_2 (Variables|Default|SetPainting_0 _returnvalue_2))
  (Rendering|Material|SetVectorParameterValue _output_get_2 "color" (select (not Team) "(R=1.000000,G=0.000000,B=0.012401,A=1.000000)" "(R=0.000000,G=0.024492,B=1.000000,A=1.000000)") :!class /Script/Engine.MaterialInstanceDynamic))

(event Custom|Respawn
  (Pawn|Components|CharacterMovement|SetMovementMode (Variables|Character|GetCharacterMovement) "MOVE_Walking" 0)
  (bind _refbase (Variables|Default|GetRefBase)
    (:then
      (bind _returnvalue (Transformation|SetActorLocation (+ (Transformation|GetActorLocation _refbase) "0.000000,0.000000,200.000000") false false))
      (Development|PrintString (Utilities|String|ToString(Boolean) _returnvalue))
      (CallFunction|ResetDoOnce))
    (:else
      (Development|PrintString "error" true true "(R=1.000000,G=0.004823,B=0.000000,A=1.000000)"))))

(event Custom|SetMaterial
  (bind _mesh (Variables|Character|GetMesh))
  (if (Variables|Default|GetIsTeamRed)
    (Rendering|Material|SetMaterial _mesh 0 "/Game/GameCore/Characters/Mannequins/Materials/Instances/Quinn/MI_Team2.MI_Team2")
    (else
      (Rendering|Material|SetMaterial _mesh 0 "/Game/GameCore/Characters/Mannequins/Materials/Instances/Quinn/MI_Team1.MI_Team1"))))

(event Custom|ResetDoOnce
  (Utilities|FlowControl|DoOnce false) ; enters at Reset
)

(event Custom|RespawnSystem
  (Utilities|FlowControl|DoOnce false
    (:Completed
      (bind _returnvalue (Game|SpawnActorfromClass "/Game/GameCore/Blueprint/BP_Decal.BP_Decal_C" (Math|Transform|MakeTransform (Transformation|GetActorLocation) "0, 0, 0" "1.250000,1.250000,1.000000") "Undefined" "MultiplyWithRoot" 0 0))
      (Rendering|Components|Decal|SetDecalMaterial (Variables|/Game/GameCore/Blueprint/BP_Decal.BP_Decal_C|GetDecal _returnvalue) (Variables|Default|GetPainting))
      (Transformation|SetActorLocation "50000.000000,50000.000000,50000.000000" false true)
      (Utilities|Time|SetTimerbyEvent (EventDispatchers|CreateEvent :!event Custom|Respawn) (Variables|Default|GetRespawnCooldown))
      (Math|Float|IncrementFloat (Variables|Default|GetRespawnCooldown)
        (:%20%20
          (Pawn|Components|CharacterMovement|SetMovementMode (Variables|Character|GetCharacterMovement) "MOVE_Custom" 0)
          (AI|Components|Blackboard|SetValueasBool (Variables|/Script/AIModule.AIController|GetBlackboard (Variables|Default|GetRef_AIC)) (Variables|Default|GetKey%20Name) false)
          (AI|Components|Blackboard|SetValueasObject (Variables|/Script/AIModule.AIController|GetBlackboard (Variables|Default|GetRef_AIC)) (Variables|Default|GetKey%20Name_0) 0))))))

(event Custom|SetAmmos
  (if (> (Variables|Default|GetAmmos) 0)
    (Math|Integer|DecrementInt (Variables|Default|GetAmmos))))

(event Custom|CustomEvent
  (bind _refbrush (Variables|Default|GetRefBrush)
    (:then
      (Default|PaintBrush _refbrush))
    (:else)))

(event EventBeginPlay
  (CallFunction|SetMaterial)
  (CallFunction|InitColorPainting (Variables|Default|GetIsTeamRed))
  (Utilities|Time|SetTimerbyEvent (EventDispatchers|CreateEvent :!event Custom|CustomEvent) 0.2 true))

(event EventTick
  (params (DeltaSeconds :type Float%20%28single-precision%29)))

(fn ConstructionScript
  (bind _mesh (Variables|Character|GetMesh))
  (if (Variables|Default|GetIsTeamRed)
    (Rendering|Material|SetMaterial _mesh 0 "/Game/GameCore/Characters/Mannequins/Materials/Instances/Quinn/MI_Team2.MI_Team2")
    (else
      (Rendering|Material|SetMaterial _mesh 0 "/Game/GameCore/Characters/Mannequins/Materials/Instances/Quinn/MI_Team1.MI_Team1"))))