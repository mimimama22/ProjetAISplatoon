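; Paintbrush weapon that stamps team-colored paint decals on surfaces and scores the painted area for red or blue.
; InitColorPainting sets the team and creates a red or blue dynamic instance of the splat material.
; PaintBrush traces a short line down from the mesh's paint socket and, on a hit, attaches a randomly sized and rolled decal.
; Each decal's area is added to the team's score in the game state and pushed to the HUD.
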(event Custom|InitColorPainting
  (params (Team :type Boolean))
  (bind _output_get (Variables|Default|SetIsTeamRed Team))
  (bind _returnvalue (Rendering|Material|CreateDynamicMaterialInstance "/Game/Market/GunSplatoon/MI_ShootSplat.MI_ShootSplat" "None" "None" :!class /Script/Engine.KismetMaterialLibrary))
  (bind _output_get_2 (Variables|Default|SetPainting _returnvalue))
  (Rendering|Material|SetVectorParameterValue _output_get_2 "color" (select _output_get "(R=1.000000,G=0.000000,B=0.012401,A=1.000000)" "(R=0.000000,G=0.024492,B=1.000000,A=1.000000)") :!class /Script/Engine.MaterialInstanceDynamic))

(event Custom|PaintBrush
  (bind _returnvalue (Math|Random|RandomFloatinRange 5e+01 1e+02))
  (bind _gamestateref (Variables|Default|GetGameStateRef))
  (bind _spawnlocation (Variables|Default|GetSpawnLocation))
  (bind _staticmesh (Variables|Default|GetStaticMesh))
  (bind _gamestateref_2 (Variables|Default|GetGameStateRef))
  (bind _gamestateref_3 (Variables|Default|GetGameStateRef))
  (bind _gamestateref_4 (Variables|Default|GetGameStateRef))
  (bind _returnvalue_2 (Transformation|GetSocketLocation _staticmesh "PaintSocket"))
  (bind _hud_ref (Variables|/Game/GameCore/Blueprint/Base/BP_CustomGameState.BP_CustomGameState_C|GetHUD_Ref _gamestateref))
  (bind _hud_ref_2 (Variables|/Game/GameCore/Blueprint/Base/BP_CustomGameState.BP_CustomGameState_C|GetHUD_Ref _gamestateref_4))
  (bind _outhit (Collision|LineTraceByChannel _returnvalue_2 (+ _returnvalue_2 "0.000000,0.000000,-50.000000") "TraceTypeQuery1" false 0 "ForOneFrame"))
  (if (.bblockinghit _outhit)
    (bind _returnvalue_3 (Class|GameplayStatics|SpawnDecalAttached (Variables|Default|GetPainting) (Math|Vector|MakeVector -75.0 _returnvalue _returnvalue) (.hitcomponent _outhit) "None" _spawnlocation (Math|Rotator|MakeRotfromX _spawnlocation) "KeepRelativeOffset" 0.0))
    (Transformation|AddRelativeRotation _returnvalue_3 (Math|Rotator|MakeRotator (Math|Random|RandomFloatinRange 0.0 3.6e+02) 0.0 0.0) false false)
    (if (Variables|Default|GetIsTeamRed)
      (bind _output_get (Variables|/Game/GameCore/Blueprint/Base/BP_CustomGameState.BP_CustomGameState_C|SetScoreRed _gamestateref_2 (+ (Variables|/Game/GameCore/Blueprint/Base/BP_CustomGameState.BP_CustomGameState_C|GetScoreRed _gamestateref_2) (* (.y (Variables|/Script/Engine.DecalComponent|GetDecalSize _returnvalue_3)) (.z (Variables|/Script/Engine.DecalComponent|GetDecalSize _returnvalue_3))))))
      (Default|SetScoreText _hud_ref (Variables|/Game/GameCore/Blueprint/UI/WBP_HUD.WBP_HUD_C|GetText_ScoreRed _hud_ref) _output_get)
      (else
        (bind _output_get_2 (Variables|/Game/GameCore/Blueprint/Base/BP_CustomGameState.BP_CustomGameState_C|SetScoreBlue _gamestateref_3 (+ (Variables|/Game/GameCore/Blueprint/Base/BP_CustomGameState.BP_CustomGameState_C|GetScoreBlue _gamestateref_3) (* (.y (Variables|/Script/Engine.DecalComponent|GetDecalSize _returnvalue_3)) (.z (Variables|/Script/Engine.DecalComponent|GetDecalSize _returnvalue_3))))))
        (Default|SetScoreText _hud_ref_2 (Variables|/Game/GameCore/Blueprint/UI/WBP_HUD.WBP_HUD_C|GetText_ScoreBlue _hud_ref_2) _output_get_2)))))

(event EventBeginPlay
  (bind _asbp_custom_game_state (Utilities|Casting|CastToBP_CustomGameState (Game|GetGameState)))
  (Variables|Default|SetGameStateRef _asbp_custom_game_state))

(fn ConstructionScript)