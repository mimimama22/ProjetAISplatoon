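; BP_SpawnBaseTeam is a team spawner actor that creates a small batch of AI units when play begins.
; On BeginPlay it loops, spawning BP_AIBase actors at its own root transform and setting their team from its IsTeamRed flag.
; Each unit is added to the RedTeam or BlueTeam array on BP_CustomGameState.
; It then receives the spawner's RefSpline and updates its material through SetMaterial.
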(event EventBeginPlay
  (for _index (range 0 3)
    (bind _returnvalue (Game|SpawnActorfromClass "/Game/GameCore/Blueprint/AI/BP_AIBase.BP_AIBase_C" (Transformation|GetWorldTransform (Variables|Default|GetDefaultSceneRoot)) "Undefined" "MultiplyWithRoot" 0 0))
    (if (Variables|Default|GetIsTeamRed)
      (Variables|/Game/GameCore/Blueprint/AI/BP_AIBase.BP_AIBase_C|SetIsTeamRed _returnvalue true)
      (Utilities|Array|Add (Variables|/Game/GameCore/Blueprint/Base/BP_CustomGameState.BP_CustomGameState_C|GetRedTeam (.AsBP%20Custom%20Game%20State (Utilities|Casting|CastToBP_CustomGameState (Game|GetGameState)))) _returnvalue)
      (else
        (Variables|/Game/GameCore/Blueprint/AI/BP_AIBase.BP_AIBase_C|SetIsTeamRed _returnvalue false)
        (Utilities|Array|Add (Variables|/Game/GameCore/Blueprint/Base/BP_CustomGameState.BP_CustomGameState_C|GetBlueTeam (.AsBP%20Custom%20Game%20State (Utilities|Casting|CastToBP_CustomGameState (Game|GetGameState)))) _returnvalue)))
    (Variables|/Game/GameCore/Blueprint/AI/BP_AIBase.BP_AIBase_C|SetRefSpline _returnvalue (Variables|Default|GetRefSpline))
    (Default|SetMaterial _returnvalue)))

(fn ConstructionScript)