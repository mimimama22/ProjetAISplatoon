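; Custom game state that runs a timed Red vs Blue match and shows the winner when time runs out.
; On BeginPlay it creates the HUD and starts a looping one-second timer to count down Timer on screen.
; At zero, EndGame swaps the HUD for an end-level widget with both scores and a colored winner text; ties go to Blue.
; The looping timer is never cleared here, and scores are only read.
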(event Custom|SetTimer
  (if (> (Variables|Default|GetTimer) 0.0)
    (bind _result (Math|Float|DecrementFloat (Variables|Default|GetTimer))
      (:%20%20
        (Default|SetTimerText (Variables|Default|GetHUD_Ref) _result)))
    (else
      (CallFunction|EndGame))))

(event Custom|EndGame
  (Widget|RemovefromParent (Variables|Default|GetHUD_Ref))
  (bind _returnvalue (UserInterface|CreateWidget "/Game/GameCore/Blueprint/UI/WBP_EndLevel.WBP_EndLevel_C"))
  (Default|SetTexts _returnvalue (Variables|Default|GetScoreBlue) (Variables|Default|GetScoreRed))
  (if (> (Variables|Default|GetScoreRed) (Variables|Default|GetScoreBlue))
    (Appearance|SetColorandOpacity (Variables|/Game/GameCore/Blueprint/UI/WBP_EndLevel.WBP_EndLevel_C|GetText_Victory _returnvalue) (Utilities|Struct|MakeSlateColor "(R=1.000000,G=0.000000,B=0.000000,A=1.000000)") :!class /Script/UMG.TextBlock)
    (Rendering|Components|TextRender|SetText (Variables|/Game/GameCore/Blueprint/UI/WBP_EndLevel.WBP_EndLevel_C|GetText_Victory _returnvalue) "Red Win")
    (else
      (Appearance|SetColorandOpacity (Variables|/Game/GameCore/Blueprint/UI/WBP_EndLevel.WBP_EndLevel_C|GetText_Victory _returnvalue) (Utilities|Struct|MakeSlateColor "(R=0.000000,G=0.000000,B=1.000000,A=1.000000)") :!class /Script/UMG.TextBlock)
      (Rendering|Components|TextRender|SetText (Variables|/Game/GameCore/Blueprint/UI/WBP_EndLevel.WBP_EndLevel_C|GetText_Victory _returnvalue) "Blue Win")))
  (UserInterface|Viewport|AddtoViewport _returnvalue 0))

(event EventBeginPlay
  (bind _returnvalue (UserInterface|CreateWidget "/Game/GameCore/Blueprint/UI/WBP_HUD.WBP_HUD_C"))
  (bind _output_get (Variables|Default|SetHUD_Ref _returnvalue))
  (UserInterface|Viewport|AddtoViewport _output_get 0)
  (Utilities|Time|SetTimerbyEvent (EventDispatchers|CreateEvent :!event Custom|SetTimer) 1.0 true))

(fn ConstructionScript)