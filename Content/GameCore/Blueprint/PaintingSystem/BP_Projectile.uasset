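; Projectile for a render-target painting system, with the painting step itself left unfinished.
; BeginPlay creates a dynamic instance of M_Painting, and the Painting event traces 50 units down but does nothing with the hit.
; PrepareDataForActor gives each material on a new actor's static mesh a dynamic instance with its own render target as "Mask".
; RenderTargets holds only the most recently prepared actor's targets.
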(event Custom|Painting
  (bind _returnvalue (Transformation|GetActorLocation))
  (bind (_outhit _returnvalue_2) (Collision|LineTraceForObjects _returnvalue (- _returnvalue "0.000000,0.000000,50.000000") (Utilities|Array|MakeArray "ObjectTypeQuery7") true 0 "None"))
  (if _returnvalue_2
    _))

(event EventBeginPlay
  (bind _returnvalue (Rendering|Material|CreateDynamicMaterialInstance "/Game/GameCore/M_Painting.M_Painting" "None" "None" :!class /Script/Engine.KismetMaterialLibrary))
  (Variables|Default|SetDMI_Painting _returnvalue))

(fn ConstructionScript)

(fn PrepareDataforActor
  (params (Actor :type Actor%20Object%20Reference) (FaceIndex :type Integer))
  (Variables|Default|SetLastActor Actor)
  (Variables|Default|SetLastFaceIndex FaceIndex)
  (if (not (Utilities|Array|ContainsItem (Variables|Default|GetActors) (Variables|Default|GetLastActor)))
    (Utilities|Array|Clear (Variables|Default|GetRenderTargets))
    (Utilities|Array|AddUnique (Variables|Default|GetActors) (Variables|Default|GetLastActor))
    (for (_array_element _array_index) (Rendering|Material|GetMaterials (Actor|GetComponentbyClass (Variables|Default|GetLastActor) "/Script/Engine.StaticMeshComponent"))
      (bind _returnvalue (Rendering|Material|CreateDynamicMaterialInstance _array_element "None" "None" :!class /Script/Engine.KismetMaterialLibrary))
      (bind _returnvalue_2 (Rendering|CreateRenderTarget2D 256 256 "RTF_RGBA16f"))
      (Rendering|Material|SetTextureParameterValue _returnvalue "Mask" _returnvalue_2)
      (Rendering|Material|SetMaterial (Actor|GetComponentbyClass (Variables|Default|GetLastActor) "/Script/Engine.StaticMeshComponent") _array_index _returnvalue)
      (Utilities|Array|AddUnique (Variables|Default|GetRenderTargets) _returnvalue_2))))